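; BP_World_Item is an inventory item placed in the world, with a mesh and an info widget.
; On BeginPlay it caches the ThirdPersonCharacter and passes the item class's default name and its Amount to WBP_World_Item.
; While that player reference is valid, Tick applies a look-at rotation to a component.
; Setting the mesh from the item class defaults is present but never runs.
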(event `self.ReceiveBeginPlay`
  (bind (_item_properties_itemname _item_properties_description _item_properties_itemtype _item_properties_itemicon _item_properties_itemmesh) (break `/Game/Dan/Inventory_System/Utilities/ST_Item` (defaults `Object` (`self.Item Signiture`))))
  ;[1 1 1] Item Inormation
  (bind _asthird_person_character (cast `/Game/AK/_CONTENTFORPACKAGE/ThirdPersonCharacter` (`GameplayStatics.GetPlayerCharacter` 0)))
  (set `self.Player Reference` _asthird_person_character)
  (bind _aswbp_world_item (cast `/Game/Dan/Inventory_System/Widgit/WBP_World_Item` (`WidgetComponent.GetUserWidgetObject` (`self.WBP Item Info`))))
  (`/Game/Dan/Inventory_System/Widgit/WBP_World_Item.Get Item Info` _aswbp_world_item _item_properties_itemname (`self.Amount`)))

(event `self.ReceiveTick`
  (params (DeltaSeconds :type "Float (single-precision)"))
  (`/Engine/EditorBlueprintResources/StandardMacros.IsValid` (`self.Player Reference`)
    (:`Is Valid`
      (`SceneComponent.K2_SetWorldRotation` (`KismetMathLibrary.FindLookAtRotation` (`SceneComponent.K2_GetComponentLocation`) (`SceneComponent.K2_GetComponentLocation`))))))

(fn `UserConstructionScript`)