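; BP_World_Items is an inventory item placed in the world, showing its mesh and an information widget.
; On BeginPlay it caches the player character and the WBP_World_Item_copy widget from its item-information component.
; It reads the class defaults of ItemSIgnature to pass the item name, along with its Amount, to the widget and to set the static mesh.
; No pickup or overlap logic is implemented here.
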(event `self.ReceiveBeginPlay`
  (bind (_item_properties_itemname _item_properties_description _item_properties_itemtype _item_properties_itemicon _item_properties_itemmesh) (break `/Game/Dan/Inventory_System/Utilities/ST_Item` (defaults `Object` (`self.Item_SIgnature`))))
  (bind _asmain_character_amin_bp (cast `/Game/MainCharacter_Amin_BP` (`GameplayStatics.GetPlayerCharacter` 0)))
  (set `self.Player_Ref` _asmain_character_amin_bp)
  (bind _aswbp_world_item_copy (cast `/Game/Dan/Inventory_System/Widgit/WBP_World_Item_copy` (`WidgetComponent.GetUserWidgetObject` (`self.WBP_Item_Information`))))
  (bind _output_get (set `self.WBP World Item Copy` _aswbp_world_item_copy))
  (`/Game/Dan/Inventory_System/Widgit/WBP_World_Item_copy.Get_Item_Information` _output_get _item_properties_itemname (`self.Amount`))
  (`StaticMeshComponent.SetStaticMesh` (`self.Item_Mesh`) _item_properties_itemmesh))

(fn `UserConstructionScript`)