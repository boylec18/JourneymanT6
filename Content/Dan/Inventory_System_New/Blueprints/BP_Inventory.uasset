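; Inventory Blueprint that stores items in an array of slots, each holding an item class and amount, sized to AmountOfSlots on BeginPlay.
; Helper functions query slots, find empty ones and find partly filled stacks of a given class.
; AddItem recursively spreads an amount across slots, stacking items flagged Usable up to MaximumStackSize and placing others one per slot, returning success and a remaining count.
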(event `self.ReceiveBeginPlay`
  (`KismetArrayLibrary.Array_Resize` (`self.Slots`) (`self.Amount_of_Slots`)))

(fn `Add_Item`
  (params (Item_Class :type "/Game/Dan/Inventory_System_New/Blueprints/Item_Classes/BP_Master_Item Class Reference") (Amount :type Integer))
  (returns (Success :type Boolean) (Remaining_Items :type Integer))
  (locals (Local_Class :type "/Game/Dan/Inventory_System_New/Blueprints/Item_Classes/BP_Master_Item Class Reference") (Local_Amount :type Integer) (Found_Index :type Integer))
  (bind _returnvalue (+ (`.Amount_5_8D0E044A4A05AFD607BE7B9AEFF7F66D` (break `/Game/Dan/Inventory_System_New/Blueprints/Structures/Struct_Inventory_Slot` (`|GetArrayItem` (`self.Slots`) (`local.Found_Index`)))) (`local.Local_Amount`)))
  (set `local.Local_Class` Item_Class)
  (set `local.Local_Amount` Amount)
  (if (`.Usable_10_B097FE6542FF9E03D5F36798C25CC43A` (break `/Game/Dan/Inventory_System_New/Blueprints/Structures/Struct_Item_information` (defaults `Object` Item_Class)))
    ;[1 1 1] Add Item True Branch(Dan) this branch searches the stack and assigns items to the stack with available space
    (bind (_success _index) (`self.Search_Free_Stack` (`local.Local_Class`)))
    (if _success
      (set `local.Found_Index` _index)
      (if (> _returnvalue (`self.Maximum_Stack_Size`))
        (set `local.Local_Amount` (- _returnvalue (`self.Maximum_Stack_Size`)))
        (`KismetArrayLibrary.Array_Set` (`self.Slots`) (`local.Found_Index`) (make `/Game/Dan/Inventory_System_New/Blueprints/Structures/Struct_Inventory_Slot` (`local.Local_Class`) (`self.Maximum_Stack_Size`)))
        (bind (_success_2 _remaining_items) (`self.Add_Item` (`local.Local_Class`) (`local.Local_Amount`)))
        (return true _remaining_items)
        (else
          (`KismetArrayLibrary.Array_Set` (`self.Slots`) (`local.Found_Index`) (make `/Game/Dan/Inventory_System_New/Blueprints/Structures/Struct_Inventory_Slot` (`local.Local_Class`) _returnvalue))
          (return false 0)))
      (else
        (bind (_success_3 _index_2) (`self.Search_Empty_Slots`))
        (if _success_3
          (bind _output_get (set `local.Found_Index` _index_2))
          (if (> (`local.Local_Amount`) (`self.Maximum_Stack_Size`))
            (`KismetArrayLibrary.Array_Set` (`self.Slots`) _output_get (make `/Game/Dan/Inventory_System_New/Blueprints/Structures/Struct_Inventory_Slot` (`local.Local_Class`) (`self.Maximum_Stack_Size`)))
            (bind (_success_4 _remaining_items_2) (`self.Add_Item` (`local.Local_Class`) (- (`local.Local_Amount`) (`self.Maximum_Stack_Size`))))
            (return true _remaining_items_2)
            (else
              (`KismetArrayLibrary.Array_Set` (`self.Slots`) (`local.Found_Index`) (make `/Game/Dan/Inventory_System_New/Blueprints/Structures/Struct_Inventory_Slot` (`local.Local_Class`) (`self.Maximum_Stack_Size`)))
              (return true 0)))
          (else
            (return false (`local.Local_Amount`))))))
    (else
      ;[1 1 1] Add Items False Branch (Dan) this branch checks if there is an empty slot and if so add this to a slot
      (bind (_success_5 _index_3) (`self.Search_Empty_Slots`))
      (if _success_5
        (bind _output_get_2 (set `local.Found_Index` _index_3))
        (`KismetArrayLibrary.Array_Set` (`self.Slots`) _output_get_2 (make `/Game/Dan/Inventory_System_New/Blueprints/Structures/Struct_Inventory_Slot` (`local.Local_Class`) 1))
        (if (> (`local.Local_Amount`) 1)
          (bind (_success_6 _remaining_items_3) (`self.Add_Item` (`local.Local_Class`) (- (`local.Local_Amount`) 1)))
          (return true _remaining_items_3)
          (else
            (return true 0)))
        (else
          (return false 0))))))

(fn `Get_Amount_At_Index`
  (params (Index :type Integer))
  (returns (Amount :type Integer))
  (return (`.Amount_5_8D0E044A4A05AFD607BE7B9AEFF7F66D` (break `/Game/Dan/Inventory_System_New/Blueprints/Structures/Struct_Inventory_Slot` (`|GetArrayItem` (`self.Slots`) Index)))))

(fn `Get_Item_Info_at_Index`
  (params (Index :type Integer))
  (returns (Empty_Slot :type Boolean) (Item_Info :type "/Game/Dan/Inventory_System_New/Blueprints/Structures/Struct_Item_information Structure") (Amount :type Integer))
  (bind (_item_class _amount) (break `/Game/Dan/Inventory_System_New/Blueprints/Structures/Struct_Inventory_Slot` (`|GetArrayItem` (`self.Slots`) Index)))
  ;[1 1 1] Get Item Information at Index (Dan) Checks whether the item has been assigned to a slot
  (if (`KismetSystemLibrary.IsValidClass` _item_class)
    (return false (defaults `Object` _item_class) _amount)
    (else
      (return true (struct) 0))))

(fn `Is_Slot_Empty`
  (params (Index :type Integer))
  (returns (Empty :type Boolean))
  ;[1 1 1] Is Slot Empty(Dan) checks if the slot is empty before assigning item
  (return (not (`KismetSystemLibrary.IsValidClass` (`.Item_Class_2_3D8C55554BE4DD253B8986BDE53E781C` (break `/Game/Dan/Inventory_System_New/Blueprints/Structures/Struct_Inventory_Slot` (`|GetArrayItem` (`self.Slots`) Index)))))))

(fn `Search_Empty_Slots`
  (returns (Success :type Boolean) (Index :type Integer))
  (locals (Local_Bool :type Boolean) (Local_Index :type Integer))
  ;[1 1 1] Search Empty Slots(Dan) Returns any empty slots
  (for (_array_element _array_index) (`self.Slots`)
    (if (not (`KismetSystemLibrary.IsValidClass` (`.Item_Class_2_3D8C55554BE4DD253B8986BDE53E781C` (break `/Game/Dan/Inventory_System_New/Blueprints/Structures/Struct_Inventory_Slot` _array_element))))
      (set `local.Local_Bool` true)
      (set `local.Local_Index` _array_index)
      (break)))
  (return (`local.Local_Bool`) (`local.Local_Index`)))

(fn `Search_Free_Stack`
  (params (Item_Class :type "/Game/Dan/Inventory_System_New/Blueprints/Item_Classes/BP_Master_Item Class Reference"))
  (returns (Success :type Boolean) (Index :type Integer))
  (locals (Local_Index :type Integer) (Local_Bool :type Boolean))
  ;[1 1 1] Search Free Stack (Dan) This function searches for the available stack with free space and adds item to it
  (for (_array_element _array_index) (`self.Slots`)
    (bind (_item_class _amount) (break `/Game/Dan/Inventory_System_New/Blueprints/Structures/Struct_Inventory_Slot` _array_element))
    (if (`KismetSystemLibrary.IsValidClass` _item_class)
      (if (and (== _item_class Item_Class) (< _amount (`self.Maximum_Stack_Size`)))
        (set `local.Local_Bool` true)
        (set `local.Local_Index` _array_index)
        (break))))
  (return (`local.Local_Bool`) (`local.Local_Index`)))

(fn `UserConstructionScript`)