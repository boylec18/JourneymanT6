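; Inventory component that currently detects what the player is looking at; its add and remove inventory functions are empty stubs.
; Every Tick it sphere-traces from the player camera along its forward vector up to InteractionRange, ignoring the owner.
; On a hit it stores the actor as LookAtActor, calls LookAtMessage on it and prints the returned message.
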(event `self.ReceiveTick`
  (params (DeltaSeconds :type "Float (single-precision)"))
  (`self.Interaction_Trace`))

(fn `Add_To_Inventory`)

(fn `Interaction_Trace`
  (bind _returnvalue (`GameplayStatics.GetPlayerCameraManager` 0))
  (bind _returnvalue_2 (`PlayerCameraManager.GetCameraLocation` _returnvalue))
  (bind (_outhit _returnvalue_3) (`KismetSystemLibrary.SphereTraceSingle` _returnvalue_2 (+ _returnvalue_2 (* (`Actor.GetActorForwardVector` _returnvalue) (`self.Interaction_Range`))) 15.0 "TraceTypeQuery3" false (`|MakeArray` (`self.GetOwner`))))
  (if _returnvalue_3
    (bind _output_get (set `self.Look_at_Actor` (`.HitActor` (`GameplayStatics.BreakHitResult` _outhit))))
    (bind _message (message `/Game/Dan/Inventory_System_New/Blueprints/BPC_Inventory_System.Look_At` _output_get))
    (`KismetSystemLibrary.PrintString` (`KismetTextLibrary.Conv_TextToString` _message))))

(fn `Remove_From_Inventory`)