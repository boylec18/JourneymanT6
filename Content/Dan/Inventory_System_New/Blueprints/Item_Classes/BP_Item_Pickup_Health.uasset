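; Health item pickup actor for the inventory system, collected by walking into its sphere.
; When the main character overlaps the sphere, it adds its configured item class and amount to that character's inventory.
; A partial add keeps the leftover amount on the pickup, while a full add destroys the actor.
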(event `self.Sphere.OnComponentBeginOverlap`
  (params (OverlappedComponent :type "PrimitiveComponent Object Reference") (OtherActor :type "Actor Object Reference") (OtherComp :type "PrimitiveComponent Object Reference") (OtherBodyIndex :type Integer) (bFromSweep :type Boolean) (SweepResult :type "HitResult Structure (by ref)"))
  (bind _asmain_character_amin_bp (cast `/Game/MainCharacter_Amin_BP` OtherActor))
  (bind _inventory_ref (`/Game/MainCharacter_Amin_BP.Inventory_Ref` _asmain_character_amin_bp))
  (`/Engine/EditorBlueprintResources/StandardMacros.IsValid` _inventory_ref
    (:`Is Valid`
      (bind (_success _remaining_items) (`/Game/Dan/Inventory_System_New/Blueprints/BP_Inventory.Add_Item` _inventory_ref (`self.Item_Class_to_Add`) (`self.Amount`)))
      (if _success
        (if (> _remaining_items 0)
          (set `self.Amount` _remaining_items)
          (else
            (`self.K2_DestroyActor`)))))))

(fn `UserConstructionScript`)