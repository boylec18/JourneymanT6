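; Ice Golem boss actor that detects the player character, stores it as its AI target and has a close-range attack event.
; A vision sphere overlap writes the Blackboard "Target" key and adds a new boss health widget on each entry; leaving clears only the key.
; ATK_CloseRange yaws the golem toward its target, then runs a debug-drawn sphere trace around itself, with the result unused.
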(event `self.SphereVision.OnComponentBeginOverlap`
  (params (OverlappedComponent :type "PrimitiveComponent Object Reference") (OtherActor :type "Actor Object Reference") (OtherComp :type "PrimitiveComponent Object Reference") (OtherBodyIndex :type Integer) (bFromSweep :type Boolean) (SweepResult :type "HitResult Structure (by ref)"))
  ;[1 1 1] Overlap Set, Get, Clear Target
  (if (!= OtherActor self)
    (bind _astesting_character_bp (cast `/Game/TestingBP/TestingCharacter_BP` OtherActor))
    (`self.SetTarget` _astesting_character_bp)
    (bind _returnvalue (`|CreateWidget` "/Game/AI/Ice_Golem_BOSS/BossHealth.BossHealth_C"))
    (`UserWidget.AddToViewport` _returnvalue 0)))

(event `self.SphereVision.OnComponentEndOverlap`
  (params (OverlappedComponent :type "PrimitiveComponent Object Reference") (OtherActor :type "Actor Object Reference") (OtherComp :type "PrimitiveComponent Object Reference") (OtherBodyIndex :type Integer))
  ;[1 1 1] Overlap Set, Get, Clear Target
  (if (== OtherActor (`self.GetTarget`))
    (`self.ClearTarget`)))

(event `ATK_CloseRange`
  (params (Target :type "Actor Object Reference"))
  (bind _returnvalue (`self.K2_GetActorLocation`))
  (bind (_returnvalue_roll _returnvalue_pitch _returnvalue_yaw) (`KismetMathLibrary.BreakRotator` (`KismetMathLibrary.FindLookAtRotation` (`self.K2_GetActorLocation`) (`self.K2_GetActorLocation` Target))))
  (`|ExecutionSequence`
    (:`then_0`
      (`/Engine/EditorBlueprintResources/StandardMacros.IsValid` Target
        (:`Is Valid`
          (`self.K2_SetActorRotation` (`KismetMathLibrary.MakeRotator` 0.0 0.0 _returnvalue_yaw)))))
    (:`then_1`
      (`KismetSystemLibrary.SphereTraceSingle` :`Start` _returnvalue :`End` _returnvalue :`Radius` 400.0 :`TraceChannel` "TraceTypeQuery2" :`DrawDebugType` "ForDuration"))))

(fn `ClearTarget`
  (`BlackboardComponent.ClearValue` (`AIBlueprintHelperLibrary.GetBlackboard` (`AIBlueprintHelperLibrary.GetAIController` self)) "Target"))

(fn `GetTarget`
  (returns (Target :type "Actor Object Reference"))
  (return (cast `Actor` (`BlackboardComponent.GetValueAsObject` (`AIBlueprintHelperLibrary.GetBlackboard` (`AIBlueprintHelperLibrary.GetAIController` self)) "Target") :!pure true)))

(fn `SetTarget`
  (params (NewTarget :type "Actor Object Reference"))
  (`BlackboardComponent.SetValueAsObject` (`AIBlueprintHelperLibrary.GetBlackboard` (`AIBlueprintHelperLibrary.GetAIController` self)) "Target" NewTarget))

(fn `UserConstructionScript`)