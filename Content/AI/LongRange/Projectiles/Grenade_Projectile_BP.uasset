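; Grenade projectile, filed under long-range AI, that explodes on contact with the main character or after a short warning flash on any other hit.
; Hits on other objects run two duplicate macros that swap the sphere's material with delays before detonation.
; BlowUpGrenade spawns an explosion emitter, runs a debug-drawn radius sphere trace and destroys the actor.
; No damage is applied here.
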(event `self.ReceiveBeginPlay`)

(event `BlowUpGrenade`
  (bind _returnvalue (`self.K2_GetActorLocation`))
  (`GameplayStatics.SpawnEmitterAtLocation` "/Game/StarterContent/Particles/P_Explosion.P_Explosion" (`.Location` (`GameplayStatics.BreakHitResult` (stale `self.Sphere.OnComponentHit` Hit))))
  (`KismetSystemLibrary.SphereTraceSingle` :`Start` _returnvalue :`End` _returnvalue :`Radius` 400.0 :`TraceChannel` "TraceTypeQuery2" :`DrawDebugType` "ForDuration")
  (`SceneComponent.SetHiddenInGame` (`self.Sphere1`) true false)
  (`self.K2_DestroyActor`))

(event `self.Sphere.OnComponentHit`
  (params (HitComponent :type "PrimitiveComponent Object Reference") (OtherActor :type "Actor Object Reference") (OtherComp :type "PrimitiveComponent Object Reference") (NormalImpulse :type "Vector Structure") (Hit :type "HitResult Structure (by ref)"))
  (if (`self.ActorHasTag` OtherActor "MainCharacter")
    (`self.BlowUpGrenade`)
    (else
      (`self.FlashingNade`))))

(event `FlashingNade`
  (bind _sphere1 (`self.Sphere1`))
  (bind _sphere1_2 (`self.Sphere1`))
  (`PrimitiveComponent.SetMaterial` _sphere1_2 0 "/Game/AI/LongRange/Projectiles/M_FlashingNade.M_FlashingNade")
  (`KismetSystemLibrary.Delay` 0.2)
  (`PrimitiveComponent.SetMaterial` _sphere1_2 0 "/Game/StarterContent/Materials/M_Basic_Wall.M_Basic_Wall")
  (`KismetSystemLibrary.Delay` 0.2)
  (`PrimitiveComponent.SetMaterial` _sphere1_2 0 "/Game/AI/LongRange/Projectiles/M_FlashingNade.M_FlashingNade")
  (`KismetSystemLibrary.Delay` 0.2)
  (`PrimitiveComponent.SetMaterial` _sphere1 0 "/Game/AI/LongRange/Projectiles/M_FlashingNade.M_FlashingNade")
  (`KismetSystemLibrary.Delay` 0.2)
  (`PrimitiveComponent.SetMaterial` _sphere1 0 "/Game/StarterContent/Materials/M_Basic_Wall.M_Basic_Wall")
  (`KismetSystemLibrary.Delay` 0.2)
  (`PrimitiveComponent.SetMaterial` _sphere1 0 "/Game/AI/LongRange/Projectiles/M_FlashingNade.M_FlashingNade")
  (`KismetSystemLibrary.Delay` 0.2)
  (`self.BlowUpGrenade`))

(fn `UserConstructionScript`)