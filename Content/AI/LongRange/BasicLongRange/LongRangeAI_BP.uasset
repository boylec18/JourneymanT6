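; Long-range AI enemy that fires projectiles, throws ice grenades and shows an alert indicator when its state changes.
; DoOnce gates rate-limit both attacks through timed resets, while the alert hides after a delay and re-arms through ResetAlert.
; Grenade pitch comes from MathShit's ballistic equation, which checks reachability and takes the lower of two launch angles toward the player character.
; On destruction it passes itself and its starting location to AddToArray for respawning.
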(event `self.ReceiveBeginPlay`
  ;[0 1 0] Begin Play
  (bind _astesting_game_mode (cast `/Game/System/TestingGameMode` (`GameplayStatics.GetGameMode`)))
  (set `self.As Testing Game Mode` _astesting_game_mode)
  (set `self.RespawnLoc` (`self.K2_GetActorLocation`)))

(event `FireAtPlayer`
  (params (Class :type "Actor Class Reference"))
  ;[1 0 0] LongRange Projectile
  (`/Engine/EditorBlueprintResources/StandardMacros.DoOnce` false :!label _label
    (:`Completed`
      (`self.SpawnProjectile` Class)
      (`KismetSystemLibrary.K2_SetTimerDelegate` (delegate `ResetFire`) 2.0))))

(event `ResetFire`
  ;[1 0 0] LongRange Projectile
  (goto _label :!via `Reset`))

(event `ThrowGrenade`
  ;[1 0 0] Throw Grenade
  (`/Engine/EditorBlueprintResources/StandardMacros.DoOnce` false :!label _label_2
    (:`Completed`
      (`self.ShootGrenade`)
      (`KismetSystemLibrary.Delay` 2.0)
      (goto _label_2 :!via `Reset`))))

(event `/Game/AI/States/AlertInterface.Change States`
  (params (`Alert State` :type "/Game/AI/States/AlertStates Enum" :default "NewEnumerator0"))
  (bind _alerted (`self.Alerted`))
  ;[1 0 0] Show Alert
  (`/Engine/EditorBlueprintResources/StandardMacros.DoOnce` false :!label _label_3
    (:`Completed`
      (`SceneComponent.SetHiddenInGame` _alerted false false)
      (`KismetSystemLibrary.Delay` 4.0)
      (`SceneComponent.SetHiddenInGame` _alerted true false))))

(event `/Game/AI/States/AlertInterface.ResetAlert`
  ;[1 0 0] Show Alert
  (goto _label_3 :!via `Reset`))

(event `self.ReceiveDestroyed`
  ;[0 1 0] Destroyed
  (`/Game/BlueprintLibary/AIFuncation_BPL.AddToArray` self (`self.RespawnLoc`)))

(fn `ShootGrenade`
  (bind _returnvalue (`self.K2_GetActorLocation`))
  (bind (_returnvalue_x _returnvalue_y _returnvalue_z) (`KismetMathLibrary.BreakVector` (`SceneComponent.K2_GetComponentLocation` (`self.GrenadeRef`))))
  (bind _returnvalue_2 (`KismetMathLibrary.Square` (`self.Velocity`)))
  (bind _outactors (`GameplayStatics.GetAllActorsOfClass` "/Game/TestingBP/TestingCharacter_BP.TestingCharacter_BP_C"))
  (for _array_element _outactors
    _)
  (bind (_returnvalue_x_2 _returnvalue_y_2 _returnvalue_z_2) (`KismetMathLibrary.BreakVector` (`self.K2_GetActorLocation` _array_element)))
  (bind _returnvalue_3 (`KismetMathLibrary.VSize2D` (`KismetMathLibrary.MakeVector2D` (- _returnvalue_x_2 _returnvalue_x) (- _returnvalue_y_2 _returnvalue_y))))
  (bind _returnvalue_4 (- (`KismetMathLibrary.Square` _returnvalue_2) (* (+ (* (`KismetMathLibrary.Square` _returnvalue_3) (`self.Gravity`)) (* (* (- _returnvalue_z_2 _returnvalue_z) _returnvalue_2) 2.0)) (`self.Gravity`))))
  (if (>= _returnvalue_4 0.0)
    (bind (_returnvalue_roll _returnvalue_pitch _returnvalue_yaw) (`KismetMathLibrary.BreakRotator` (`KismetMathLibrary.FindLookAtRotation` _returnvalue (`self.K2_GetActorLocation` _array_element))))
    (bind _returnvalue_5 (`KismetMathLibrary.Sqrt` _returnvalue_4))
    (bind _returnvalue_6 (* _returnvalue_3 (`self.Gravity`)))
    (`|SpawnActorFromClass` "/Game/AI/LongRange/Projectiles/IceGrenade.IceGrenade_C" (`KismetMathLibrary.MakeTransform` _returnvalue (`KismetMathLibrary.MakeRotator` _returnvalue_roll (`KismetMathLibrary.FMin` (`KismetMathLibrary.DegAtan` (/ (+ _returnvalue_5 _returnvalue_2) _returnvalue_6)) (`KismetMathLibrary.DegAtan` (/ (- _returnvalue_2 _returnvalue_5) _returnvalue_6))) _returnvalue_yaw)) "Undefined" "OverrideRootScale" null null)))

(fn `SpawnProjectile`
  (params (Class :type "Actor Class Reference"))
  (bind _spawnlocation (`self.SpawnLocation`))
  (`|SpawnActorFromClass` Class (`KismetMathLibrary.MakeTransform` (`SceneComponent.K2_GetComponentLocation` _spawnlocation) (`SceneComponent.K2_GetComponentRotation` _spawnlocation) (0.5 0.5 0.5)) "AdjustIfPossibleButAlwaysSpawn" "OverrideRootScale" null null))

(fn `UserConstructionScript`)