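; Interactable sign that shows its SignText to the player in an on-screen widget.
; Interact uses a FlipFlop: the first use creates the sign widget, passing it the text and a None movement mode, and adds it to the viewport.
; The next use removes the widget, then restores the player character's Walking mode and re-enables input.
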(event `/Game/Interaction/InteractionSystem/Interact_BPI.Interact`
  (`/Engine/EditorBlueprintResources/StandardMacros.FlipFlop`
    (:`A`
      (bind _returnvalue (`/Game/BlueprintLibary/SignUpdateLibary.AddSignWidget` (`self.SignText`)))
      (`UserWidget.AddToViewport` _returnvalue 0))
    (:`B`
      (`Widget.RemoveFromParent` _returnvalue)
      (`CharacterMovementComponent.SetMovementMode` (`Character.CharacterMovement` (`GameplayStatics.GetPlayerCharacter` 0)) "MOVE_Walking" 0)
      (`self.EnableInput` (`GameplayStatics.GetPlayerCharacter` 0) (`GameplayStatics.GetPlayerController` 0)))))

(fn `UserConstructionScript`
  (`parent.UserConstructionScript`))