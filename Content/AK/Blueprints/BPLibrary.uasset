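; Blueprint library of helper functions for damage calculation and ID lookups.
; CalcDamage subtracts receiving defense from attacker power, clamps the difference, then applies random variance around DefaultVariance and truncates, so results can fall outside the clamp.
; GetColLibrary and GetPsychLibrary use switches to map integer IDs to Col and Psych values.
; Unmatched IDs fall back to the last Col entry and the first Psych entry.
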(fn `CalcDamage`
  (params (AttackerPWR :type Integer :default 0) (ReceivingDEF :type Integer))
  (returns (OutputDamage :type Integer))
  (locals (DefaultVariance :type "Float (double-precision)" :default 0.2))
  (bind _defaultvariance (`local.DefaultVariance`))
  (return (`KismetMathLibrary.FTrunc` (* (`KismetMathLibrary.Clamp` (- (* AttackerPWR 1) (* ReceivingDEF 1)) 1 9999) (`KismetMathLibrary.RandomFloatInRange` (- 1.0 _defaultvariance) (+ _defaultvariance 1.0))))))

(fn `GetColLibrary`
  (params (ColID :type Integer))
  (returns (OutputColor :type "Color Structure"))
  (locals (Col_0 :type "Color Structure" :default (struct :`B` 53 :`R` 255 :`A` 1)) (Col_1 :type "Color Structure" :default (struct :`B` 57 :`R` 186 :`A` 1)) (Col_2 :type "Color Structure" :default (struct :`G` 158 :`R` 255 :`A` 1)) (Col_3 :type "Color Structure" :default (struct :`G` 233 :`R` 255 :`A` 1)) (Col_4 :type "Color Structure" :default (struct :`G` 255 :`R` 208 :`A` 1)) (Col_5 :type "Color Structure" :default (struct :`G` 132 :`R` 27 :`A` 1)) (Col_6 :type "Color Structure" :default (struct :`B` 169 :`G` 19 :`A` 1)) (Col_7 :type "Color Structure" :default (struct :`B` 138 :`G` 160 :`R` 47 :`A` 1)) (Col_8 :type "Color Structure" :default (struct :`B` 200 :`G` 255 :`A` 1)) (Col_9 :type "Color Structure" :default (struct :`B` 255 :`R` 100 :`A` 1)) (Col_10 :type "Color Structure" :default (struct :`B` 255 :`R` 170 :`A` 1)) (Col_11 :type "Color Structure" :default (struct :`B` 145 :`R` 87 :`A` 1)) (Col_12 :type "Color Structure" :default (struct :`G` 56 :`R` 140 :`A` 1)) (Col_13 :type "Color Structure" :default (struct :`B` 67 :`G` 42 :`R` 42 :`A` 1)) (Col_14 :type "Color Structure" :default (struct :`B` 255 :`G` 255 :`R` 255 :`A` 1)) (Col_15 :type "Color Structure" :default (struct :`B` 192 :`G` 221 :`R` 255 :`A` 1)) (Col_16 :type "Color Structure" :default (struct :`B` 244 :`G` 166 :`R` 255 :`A` 1)) (Col_17 :type "Color Structure" :default (struct :`B` 236 :`R` 255 :`A` 1)) (Col_18 :type "Color Structure" :default (struct :`B` 71 :`G` 255 :`A` 1)) (Col_19 :type "Color Structure" :default (struct :`B` 255 :`G` 188 :`R` 225 :`A` 1)) (Col_20 :type "Color Structure" :default (struct :`B` 140 :`G` 164 :`R` 255 :`A` 1)) (Col_21 :type "Color Structure" :default (struct :`B` 187 :`G` 187 :`R` 195 :`A` 1)))
  (switch `int` ColID
    (:`Default`
      _)
    (:`0`
      (return (`local.Col_0`)))
    (:`1`
      (return (`local.Col_1`)))
    (:`2`
      (return (`local.Col_2`)))
    (:`3`
      (return (`local.Col_3`)))
    (:`4`
      (return (`local.Col_4`)))
    (:`5`
      (return (`local.Col_5`)))
    (:`6`
      (return (`local.Col_6`)))
    (:`7`
      (return (`local.Col_7`)))
    (:`8`
      (return (`local.Col_8`)))
    (:`9`
      (return (`local.Col_9`)))
    (:`10`
      (return (`local.Col_10`)))
    (:`11`
      (return (`local.Col_11`)))
    (:`12`
      (return (`local.Col_12`)))
    (:`13`
      (return (`local.Col_13`)))
    (:`14`
      (return (`local.Col_14`)))
    (:`15`
      (return (`local.Col_15`)))
    (:`16`
      (return (`local.Col_16`)))
    (:`17`
      (return (`local.Col_17`)))
    (:`18`
      (return (`local.Col_18`)))
    (:`19`
      (return (`local.Col_19`)))
    (:`20`
      (return (`local.Col_20`)))
    (:`21`
      _))
  (return (`local.Col_21`)))

(fn `GetPsychLibrary`
  (params (PsychID :type Integer))
  (returns (Psych :type "/Game/AK/Enumerations/EPsychs Enum"))
  (switch `int` PsychID
    (:`Default`
      _)
    (:`0`
      _)
    (:`1`
      (return "NewEnumerator1"))
    (:`2`
      (return "NewEnumerator2"))
    (:`3`
      (return "NewEnumerator3")))
  (return "NewEnumerator0"))