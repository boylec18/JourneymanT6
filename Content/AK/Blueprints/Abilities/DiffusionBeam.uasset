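; Diffusion Beam is a held ability that projects a Niagara beam from the caster to its target, with montage and audio.
; A capsule is sized to the beam's length and collects overlapped EnemyOLD actors as collateral targets, but the damage loop is disconnected.
; While held, Tick updates the beam and drains the ability value, triggering burnout at zero; otherwise it tracks inactive time.
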(event `self.ReceiveTick`
  (params (DeltaSeconds :type "Float (single-precision)"))
  ;[0.4152 0.9602 1] Event Tick
  (`parent.ReceiveTick` DeltaSeconds)
  (if (not (`self.IsBurntOut?`))
    (`|ExecutionSequence`
      (:`then_0`
        (if (`self.ButtonPressed`)
          (set `self.T_TimeInactive` 0.0)
          (set `self.AbilityCurrentValue` (- (`self.AbilityCurrentValue`) (`GameplayStatics.GetWorldDeltaSeconds`)))
          (`self.UpdateBeamLocation`)
          (else
            (set `self.T_TimeInactive` (+ (`self.T_TimeInactive`) (`GameplayStatics.GetWorldDeltaSeconds`))))))
      (:`then_1`
        (if (<= (`self.AbilityCurrentValue`) 0.0)
          (`self.StopAttack`)
          (`self.XXX BeginBurnout`)
          (`AudioComponent.Stop` (`self.Audio`)))))))

(event `self.Interupt Action`
  ;[1 1 1] Interupt Action
  (`self.StopPsychInput`)
  (`self.StopAttack`)
  (set `self.ButtonPressed` false))

(event `self.Capsule.OnComponentBeginOverlap`
  (params (OverlappedComponent :type "PrimitiveComponent Object Reference") (OtherActor :type "Actor Object Reference") (OtherComp :type "PrimitiveComponent Object Reference") (OtherBodyIndex :type Integer) (bFromSweep :type Boolean) (SweepResult :type "HitResult Structure (by ref)"))
  ;[1 1 1] Get enemies collided withh beam hitbox
  (if (`self.ButtonPressed`)
    (bind _asenemy_old (cast `/Game/AK/_CONTENTFORPACKAGE/EnemyOLD` OtherActor))
    (`KismetArrayLibrary.Array_AddUnique` (`self.CollateralTargets`) _asenemy_old)
    (`self.BeginDamagingEnemy`)))

(event `self.Capsule.OnComponentEndOverlap`
  (params (OverlappedComponent :type "PrimitiveComponent Object Reference") (OtherActor :type "Actor Object Reference") (OtherComp :type "PrimitiveComponent Object Reference") (OtherBodyIndex :type Integer))
  ;[1 1 1] Get enemies collided withh beam hitbox
)

(event `BeginDamagingEnemy`
  ;[1 1 1] Beam damage enemies loop
)

(fn `StartPsychInput`
  (bind _caster (`self.Caster`))
  (bind _returnvalue (`SceneComponent.K2_GetComponentLocation` (`self.DefaultSceneRoot`)))
  (set `self.ButtonPressed` true)
  (`self.SetCasterAttacking` true)
  (`|ExecutionSequence`
    (:`then_0`
      ;[1 1 1] Handle Beam Projection (Switch to event later?)
      (`/Game/MainCharacter_Amin_BP.FaceTarget` _caster)
      (`Character.PlayAnimMontage` _caster null 1.0 "None")
      (bind _newparam (`/Game/MainCharacter_Amin_BP.GetTargetLocation` (`self.Caster`)))
      (`NiagaraComponent.SetNiagaraVariableVec3` (`self.Niagara`) "beamEnd" _newparam)
      (`SceneComponent.SetVisibility` (`self.Niagara`) true false)
      (`CapsuleComponent.SetCapsuleHalfHeight` (`self.Capsule`) (/ (`KismetMathLibrary.Vector_Distance` _returnvalue _newparam) 2.0) true)
      (`SceneComponent.K2_SetWorldLocation` (`self.Scene`) (/ (+ _returnvalue _newparam) 2.0) false false)
      (`PrimitiveComponent.SetCollisionEnabled` (`self.Capsule`) "QueryOnly")
      (`AudioComponent.Play` (`self.Audio`) 0.0))))

(fn `StopPsychInput`
  (set `self.ButtonPressed` false)
  (`self.SetCasterAttacking` false)
  (`SceneComponent.SetVisibility` (`self.Niagara`) false false)
  (`Character.StopAnimMontage` (`self.Caster`) null)
  (`PrimitiveComponent.SetCollisionEnabled` (`self.Capsule`) "NoCollision")
  (`CapsuleComponent.SetCapsuleHalfHeight` (`self.Capsule`) 0.0 true)
  (bind _newparam (`/Game/MainCharacter_Amin_BP.GetTargetLocation` (`self.Caster`)))
  (`SceneComponent.K2_SetWorldLocation` (`self.Scene`) _newparam false false)
  (`AudioComponent.Stop` (`self.Audio`))
  (`KismetArrayLibrary.Array_Clear` (`self.CollateralTargets`)))

(fn `UpdateBeamLocation`
  (`/Game/MainCharacter_Amin_BP.FaceTarget` (`self.Caster`))
  (bind _newparam (`/Game/MainCharacter_Amin_BP.GetTargetLocation` (`self.Caster`)))
  (`NiagaraComponent.SetNiagaraVariableVec3` (`self.Niagara`) "beamEnd" _newparam)
  (`CapsuleComponent.SetCapsuleHalfHeight` (`self.Capsule`) (/ (`KismetMathLibrary.Vector_Distance` (`SceneComponent.K2_GetComponentLocation` (`self.DefaultSceneRoot`)) _newparam) 2.0) true))

(fn `UserConstructionScript`
  (`parent.UserConstructionScript`))