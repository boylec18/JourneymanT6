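; EnergyRounds is an ability Blueprint for a projectile attack triggered through psych input, apparently unfinished or disabled.
; StartPsychInput resets an inactivity timer that Tick accumulates, calls FireRound and pulses the PinGauge UI.
; FireRound is empty: the gauge drain, caster facing and montage, projectile setup and sound sit in disconnected chains that never run.
; An environment query (EQS) actor lookup is also left unwired.
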(event `self.ReceiveTick`
  (params (DeltaSeconds :type "Float (single-precision)"))
  (`parent.ReceiveTick` DeltaSeconds)
  (set `self.T_TimeInactive` (+ (`self.T_TimeInactive`) DeltaSeconds)))

(event `Fire Round`
  ;[1 1 1] Projectile fire
)

(fn `StartPsychInput`
  (`parent.StartPsychInput`)
  (set `self.T_TimeInactive` 0.0)
  (`self.Fire Round`)
  (`/Game/AK/UI/PinGauge.PlayPulse` (cast `/Game/AK/UI/PinGauge` (`self.GaugeUI`) :!pure true)))

(fn `UserConstructionScript`
  (`parent.UserConstructionScript`))