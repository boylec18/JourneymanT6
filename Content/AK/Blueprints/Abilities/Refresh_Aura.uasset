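; Refresh_Aura is a held-input psych ability that drains its ability value while active; no aura effect is implemented in this graph.
; StartPsychInput sets ButtonPressed, and Tick then drains the value by delta time, or accumulates inactive time when released, unless burnt out.
; Reaching zero stops the attack and audio and begins burnout.
; Releasing or interrupting clears the input and stops audio, with release also ending the caster's attack state and montage.
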(event `self.ReceiveTick`
  (params (DeltaSeconds :type "Float (single-precision)"))
  ;[0.3434 0.9801 1] Event Tick
  (`parent.ReceiveTick` DeltaSeconds)
  (if (not (`self.IsBurntOut?`))
    (`|ExecutionSequence`
      (:`then_0`
        (if (`self.ButtonPressed`)
          (set `self.T_TimeInactive` 0.0)
          (set `self.AbilityCurrentValue` (- (`self.AbilityCurrentValue`) (`GameplayStatics.GetWorldDeltaSeconds`)))
          (else
            (set `self.T_TimeInactive` (+ (`self.T_TimeInactive`) (`GameplayStatics.GetWorldDeltaSeconds`))))))
      (:`then_1`
        (if (<= (`self.AbilityCurrentValue`) 0.0)
          (`self.StopAttack`)
          (`self.XXX BeginBurnout`)
          (`AudioComponent.Stop` (`self.Audio`)))))))

(event `self.Interupt Action`
  (`self.StopPsychInput`)
  (`self.StopAttack`)
  (`AudioComponent.Stop` (`self.Audio`))
  (set `self.ButtonPressed` false))

(fn `StartPsychInput`
  (set `self.ButtonPressed` true))

(fn `StopPsychInput`
  (set `self.ButtonPressed` false)
  (`self.SetCasterAttacking` false)
  (`Character.StopAnimMontage` (`self.Caster`) null)
  (`AudioComponent.Stop` (`self.Audio`)))

(fn `UserConstructionScript`
  (`parent.UserConstructionScript`))