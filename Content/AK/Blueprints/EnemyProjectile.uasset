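; EnemyProjectile is an enemy-fired projectile actor that damages the ThirdPersonCharacter on overlap.
; Setup stores the damage value and caster, which the collision overlap passes to the character's TakeDamage with no blowdown.
; A destruction flag limits it to one hit, after which it deactivates particles, hides the mesh, zeroes velocity and destroys itself following a short delay.
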(event `self.Collision.OnComponentBeginOverlap`
  (params (OverlappedComponent :type "PrimitiveComponent Object Reference") (OtherActor :type "Actor Object Reference") (OtherComp :type "PrimitiveComponent Object Reference") (OtherBodyIndex :type Integer) (bFromSweep :type Boolean) (SweepResult :type "HitResult Structure (by ref)"))
  (bind _asthird_person_character (cast `/Game/AK/_CONTENTFORPACKAGE/ThirdPersonCharacter` OtherActor))
  (`KismetSystemLibrary.PrintString` "ENEMY PROJECTILE HIT")
  (if (not (`self.IsBeingDestroyed`))
    (set `self.IsBeingDestroyed` true)
    (`ActorComponent.Deactivate` (`self.Particles`))
    (`/Game/AK/_CONTENTFORPACKAGE/ThirdPersonCharacter.TakeDamage` _asthird_person_character (`self.DamageValue`) false (`self.Caster`))
    (`SceneComponent.SetVisibility` (`self.StaticMeshComponent`) false false)
    (`ProjectileMovementComponent.SetVelocityInLocalSpace` (`self.ProjectileMovement`) (0.0 0.0 0.0))
    (`KismetSystemLibrary.Delay` 2.0)
    (`self.K2_DestroyActor`)))

(fn `Setup`
  (params (DamageValue :type Integer) (Caster :type "/Game/AK/_CONTENTFORPACKAGE/Enemy Object Reference"))
  (set `self.DamageValue` DamageValue)
  (set `self.Caster` Caster))

(fn `UserConstructionScript`)