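; Test player character prototype with health, death, freeze, dodge and interaction, plus a HUD created at BeginPlay.
; Debug keys adjust HP and toggle freeze, which lowers max HP; any positive damage zeroes the clamped health check, disabling movement and input.
; Space plays a dodge montage with hop and forward launches, locked until completion.
; InteractHitBox overlaps with tagged actors open a gate letting Interact input send InteractMessage.
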(event `self.ReceiveBeginPlay`
  (`|ExecutionSequence`
    (:`then_0`
      (bind _returnvalue (`|CreateWidget` "/Game/Ennis/Interaction/Widgets/InteractText_Widget.InteractText_Widget_C"))
      (set `self.InteractWidget` _returnvalue))
    (:`then_1`
      (bind _returnvalue_2 (`|CreateWidget` "/Game/Ennis/Interaction/Widgets/HUD.HUD_C"))
      (`UserWidget.AddToViewport` _returnvalue_2 0))))

(event `self.ReceiveAnyDamage`
  (params (Damage :type "Float (single-precision)") (DamageType :type "DamageType Object Reference") (InstigatedBy :type "Controller Object Reference") (DamageCauser :type "Actor Object Reference"))
  (bind _output_get (set `self.CurrentHP` (- 0.0 Damage)))
  (if (== (`KismetMathLibrary.FClamp` _output_get) 0.0)
    (`/Engine/EditorBlueprintResources/StandardMacros.DoOnce` false
      (:`Completed`
        (set `self.IsDead` true)
        (`self.Dead`)))))

(event `self.ReceiveTick`
  (params (DeltaSeconds :type "Float (single-precision)")))

(event `Key|H`
  (params (Key :type "Key Structure"))
  (bind _currenthp (`self.CurrentHP`))
  ;[1 1 1] Testing HP
  (:`Pressed`
    (if (< _currenthp (`self.MaxHP`))
      (set `self.CurrentHP` (+ _currenthp 0.1)))))

(event `Key|J`
  (params (Key :type "Key Structure"))
  ;[1 1 1] Testing HP
  (:`Pressed`
    (set `self.CurrentHP` (- (`self.CurrentHP`) 1.0))))

(event `self.InteractHitBox.OnComponentBeginOverlap`
  (params (OverlappedComponent :type "PrimitiveComponent Object Reference") (OtherActor :type "Actor Object Reference") (OtherComp :type "PrimitiveComponent Object Reference") (OtherBodyIndex :type Integer) (bFromSweep :type Boolean) (SweepResult :type "HitResult Structure (by ref)"))
  ;[1 0.6582 0] Interaction Control
  (`/Engine/EditorBlueprintResources/StandardMacros.IsValid` OtherActor
    (:`Is Valid`
      (if (or (`self.ActorHasTag` OtherActor "Interactable") (`self.ActorHasTag` OtherActor "PickUp"))
        (goto _label :!via `Open`)))))

(event `self.InteractHitBox.OnComponentEndOverlap`
  (params (OverlappedComponent :type "PrimitiveComponent Object Reference") (OtherActor :type "Actor Object Reference") (OtherComp :type "PrimitiveComponent Object Reference") (OtherBodyIndex :type Integer))
  ;[1 0.6582 0] Interaction Control
  (goto _label :!via `Close`))

(event `InputAction|Interact`
  (params (Key :type "Key Structure"))
  ;[1 0.6582 0] Interaction Control
  (:`Pressed`
    (`/Engine/EditorBlueprintResources/StandardMacros.Gate` true :!label _label
      (:`Exit`
        (message `/Game/Ennis/Interaction/InteractionSystem/Interact_BPI.Interact` (stale `self.InteractHitBox.OnComponentBeginOverlap` OtherActor))))))

(event `Key|G`
  (params (Key :type "Key Structure"))
  ;[1 1 1] Testing freeze mechanic.
  (:`Pressed`
    (set `self.IsFrozen` false)
    (if (`self.IsFrozen`) :!label _label_2
      (if (> (`self.CurrentHP`) 2.0)
        (set `self.CurrentHP` 2.0))
      (set `self.MaxHP` (- (`self.MaxHP`) 1.0))
      (else
        (set `self.MaxHP` 3.0)))))

(event `Key|F`
  (params (Key :type "Key Structure"))
  ;[1 1 1] Testing freeze mechanic.
  (:`Released`
    (set `self.IsFrozen` true)
    (goto _label_2)))

(event `Key|SpaceBar`
  (params (Key :type "Key Structure"))
  (:`Pressed`
    (`/Engine/EditorBlueprintResources/StandardMacros.DoOnce` false :!label _label_3
      (:`Completed`
        (`|PlayMontage` (`self.Mesh`) "/Game/Character/Animations/Dodge_Montage.Dodge_Montage"
          (:`then`
            (`self.LaunchCharacter` (0.0 0.0 200.0))
            (`KismetSystemLibrary.Delay` 0.05)
            (`self.LaunchCharacter` (* (`KismetMathLibrary.GetForwardVector` (`self.K2_GetActorRotation`)) (`self.DodgeDisance`))))
          (:`OnCompleted`
            (`self.Reset Roll`)))))))

(event `Reset Roll`
  (goto _label_3 :!via `Reset`))

(event `self.DamageHitbox.OnComponentHit`
  (params (HitComponent :type "PrimitiveComponent Object Reference") (OtherActor :type "Actor Object Reference") (OtherComp :type "PrimitiveComponent Object Reference") (NormalImpulse :type "Vector Structure") (Hit :type "HitResult Structure (by ref)"))
  (cast `/Game/Ennis/TestingBP/TestingCharacter_BP` OtherActor))

(fn `Dead`
  (`CharacterMovementComponent.DisableMovement` (`self.CharacterMovement`))
  (`self.DisableInput` (`GameplayStatics.GetPlayerCharacter` 0) (`GameplayStatics.GetPlayerController` 0)))

(fn `UserConstructionScript`)