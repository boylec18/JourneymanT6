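; Interactable chest actor that bursts out coins when the player interacts with it.
; A sphere overlap with TestingCharacter_BP shows or hides the interact widget.
; The Interact event runs once, destroys the widget and starts a looping timer.
; Each tick spawns a BP_Coins actor at a random offset above the chest, until a counter hits its limit and clears the timer.
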(event `/Game/Ennis/Interaction/InteractionSystem/Interact_BPI.Interact`
  (`/Engine/EditorBlueprintResources/StandardMacros.DoOnce` false
    (:`Completed`
      (`ActorComponent.K2_DestroyComponent` (`self.InteractWidget`))
      (bind _returnvalue (`KismetSystemLibrary.K2_SetTimerDelegate` (delegate `SpawnCoins`) 0.1 true))
      (set `self.SpawnCoinTimer` _returnvalue))))

(event `SpawnCoins`
  (bind _returnvalue (`KismetMathLibrary.RandomFloatInRange` 0.0 100.0))
  (bind _coinstospawn (`self.CoinsToSpawn`))
  (bind (_returnvalue_x _returnvalue_y _returnvalue_z) (`KismetMathLibrary.BreakVector` (+ (+ (`self.K2_GetActorLocation`) (0.0 0.0 100.0)) (`KismetMathLibrary.MakeVector` _returnvalue _returnvalue _returnvalue))))
  (if (== _coinstospawn 10)
    (`KismetSystemLibrary.K2_ClearAndInvalidateTimerHandle` (`self.SpawnCoinTimer`))
    (set `self.CoinsToSpawn` 0)
    (else
      (`/Engine/EditorBlueprintResources/StandardMacros.IncrementInt` _coinstospawn
        (:`  `
          (`|SpawnActorFromClass` "/Game/Ennis/BP_Coins.BP_Coins_C" (`KismetMathLibrary.MakeTransform` (`KismetMathLibrary.MakeVector` _returnvalue_x _returnvalue_y _returnvalue_z)) "AlwaysSpawn" "OverrideRootScale" null null))))))

(event `self.Sphere.OnComponentBeginOverlap`
  (params (OverlappedComponent :type "PrimitiveComponent Object Reference") (OtherActor :type "Actor Object Reference") (OtherComp :type "PrimitiveComponent Object Reference") (OtherBodyIndex :type Integer) (bFromSweep :type Boolean) (SweepResult :type "HitResult Structure (by ref)"))
  (bind _interactwidget (`self.InteractWidget`))
  (cast `/Game/Ennis/TestingBP/TestingCharacter_BP` OtherActor)
  (`/Engine/EditorBlueprintResources/StandardMacros.IsValid` _interactwidget
    (:`Is Valid`
      (`SceneComponent.SetHiddenInGame` _interactwidget false false))))

(event `self.Sphere.OnComponentEndOverlap`
  (params (OverlappedComponent :type "PrimitiveComponent Object Reference") (OtherActor :type "Actor Object Reference") (OtherComp :type "PrimitiveComponent Object Reference") (OtherBodyIndex :type Integer))
  (bind _interactwidget (`self.InteractWidget`))
  (cast `/Game/Ennis/TestingBP/TestingCharacter_BP` OtherActor)
  (`/Engine/EditorBlueprintResources/StandardMacros.IsValid` _interactwidget
    (:`Is Valid`
      (`SceneComponent.SetHiddenInGame` _interactwidget true false))))

(fn `UserConstructionScript`
  (`parent.UserConstructionScript`))