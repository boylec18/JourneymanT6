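; Ice Golem boss character that targets the player and performs a close-range attack.
; Sphere vision overlap writes the main character into the AI Blackboard Target key and adds a boss health widget; the target clears when it leaves.
; The close-range attack event calls a yaw look-at, then a sphere trace around the boss that applies damage and spawns an ice Niagara hit effect on Player-tagged actors.
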(event `self.ReceiveBeginPlay`
  ;[0 1 0] BeginPlay
  (set `self.Health` (`self.MaxHealth`)))

(event `self.SphereVision.OnComponentBeginOverlap`
  (params (OverlappedComponent :type "PrimitiveComponent Object Reference") (OtherActor :type "Actor Object Reference") (OtherComp :type "PrimitiveComponent Object Reference") (OtherBodyIndex :type Integer) (bFromSweep :type Boolean) (SweepResult :type "HitResult Structure (by ref)"))
  ;[0 1 0] Overlap Set, Get, Clear Target
  (if (!= OtherActor self)
    (bind _asmain_character_amin_bp (cast `/Game/MainCharacter_Amin_BP` OtherActor))
    (`self.SetTarget` _asmain_character_amin_bp)
    (bind _returnvalue (`|CreateWidget` "/Game/Ennis/Ice_Golem_BOSS/BossHealth.BossHealth_C"))
    (`UserWidget.AddToViewport` _returnvalue 0)))

(event `self.SphereVision.OnComponentEndOverlap`
  (params (OverlappedComponent :type "PrimitiveComponent Object Reference") (OtherActor :type "Actor Object Reference") (OtherComp :type "PrimitiveComponent Object Reference") (OtherBodyIndex :type Integer))
  ;[0 1 0] Overlap Set, Get, Clear Target
  (if (== OtherActor (`self.GetTarget`))
    (`self.ClearTarget`)))

(event `ATK_CloseRange`
  (params (Target :type "Actor Object Reference"))
  (bind _returnvalue (`self.K2_GetActorLocation`))
  (bind (_returnvalue_roll _returnvalue_pitch _returnvalue_yaw) (`KismetMathLibrary.BreakRotator` (`KismetMathLibrary.FindLookAtRotation` (`self.K2_GetActorLocation`) (`self.K2_GetActorLocation` Target))))
  ;[1 0 0] Attack
  (`|ExecutionSequence`
    (:`then_0`
      (`/Engine/EditorBlueprintResources/StandardMacros.IsValid` Target
        (:`Is Valid`
          (`self.K2_SetActorRotation` (`KismetMathLibrary.MakeRotator` 0.0 0.0 _returnvalue_yaw)))))
    (:`then_1`
      (bind (_outhit _returnvalue_2) (`KismetSystemLibrary.SphereTraceSingleForObjects` :`Start` _returnvalue :`End` _returnvalue :`Radius` 500.0 :`ObjectTypes` (`self.Object Types`) :`DrawDebugType` "ForDuration"))
      (if _returnvalue_2
        (bind (_bblockinghit _binitialoverlap _time _distance _location _impactpoint _normal _impactnormal _physmat _hitactor) (`GameplayStatics.BreakHitResult` _outhit))
        (if (`self.ActorHasTag` _hitactor "Player")
          (`NiagaraFunctionLibrary.SpawnSystemAtLocation` "/Game/ParticleSystems/VFX/AdvancedMagicFX12/particles/Niagara/NS_ky_hit_ice.NS_ky_hit_ice" (`self.K2_GetActorLocation` _hitactor) (struct) (3.0 3.0 3.0))
          (`GameplayStatics.ApplyDamage` _hitactor 1.0 null self))))))

(fn `ClearTarget`
  (`BlackboardComponent.ClearValue` (`AIBlueprintHelperLibrary.GetBlackboard` (`AIBlueprintHelperLibrary.GetAIController` self)) "Target"))

(fn `GetTarget`
  (returns (Target :type "Actor Object Reference"))
  (return (cast `Actor` (`BlackboardComponent.GetValueAsObject` (`AIBlueprintHelperLibrary.GetBlackboard` (`AIBlueprintHelperLibrary.GetAIController` self)) "Target") :!pure true)))

(fn `SetTarget`
  (params (NewTarget :type "Actor Object Reference"))
  (`BlackboardComponent.SetValueAsObject` (`AIBlueprintHelperLibrary.GetBlackboard` (`AIBlueprintHelperLibrary.GetAIController` self)) "Target" NewTarget))

(fn `UserConstructionScript`)