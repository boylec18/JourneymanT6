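; Frost slime enemy that telegraphs a jump attack with a material flash, then hops and launches itself forward.
; While attacking, looping timers turn it toward the player and sphere-trace to damage the player, with a cooldown.
; A timer keeps clearing the AI blackboard's alert flag, and separate events show a brief alert indicator once until reset.
; On destruction it passes itself and its spawn location to AddToArray.
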(event `self.ReceiveBeginPlay`
  (`parent.ReceiveBeginPlay`)
  (`KismetSystemLibrary.K2_SetTimerDelegate` (delegate `AttackSphere`) 0.09 true)
  (set `self.SpawnLocation` (`self.K2_GetActorLocation`))
  (`KismetSystemLibrary.K2_SetTimerDelegate` (delegate `Look At Player`) 0.1 true)
  (`KismetSystemLibrary.K2_SetTimerDelegate` (delegate `CheckAlert`) 0.1 true))

(event `AttackSphere`
  (bind _returnvalue (`self.K2_GetActorLocation`))
  (if (`self.IsAttacking`)
    (bind (_outhit _returnvalue_2) (`KismetSystemLibrary.SphereTraceSingleForObjects` _returnvalue _returnvalue 100.0 (`|MakeArray` "ObjectTypeQuery3" :!type "EObjectTypeQuery Enum")))
    (if _returnvalue_2
      (bind (_bblockinghit _binitialoverlap _time _distance _location _impactpoint _normal _impactnormal _physmat _hitactor) (`GameplayStatics.BreakHitResult` _outhit))
      (if (`self.ActorHasTag` _hitactor "Player")
        (`/Engine/EditorBlueprintResources/StandardMacros.DoOnce` false :!label _label
          (:`Completed`
            (`GameplayStatics.ApplyDamage` _hitactor 1.0 null self)
            (`KismetSystemLibrary.Delay` 1.0)
            (`self.ResetDmg`)))))))

(event `ResetDmg`
  (goto _label :!via `Reset`))

(event `Look At Player`
  (bind (_returnvalue_roll _returnvalue_pitch _returnvalue_yaw) (`KismetMathLibrary.BreakRotator` (`KismetMathLibrary.FindLookAtRotation` (`self.K2_GetActorLocation`) (`self.K2_GetActorLocation` (`GameplayStatics.GetPlayerCharacter` 0)))))
  (if (`self.IsAttacking`)
    (`self.K2_SetActorRotation` (`KismetMathLibrary.MakeRotator` 0.0 0.0 _returnvalue_yaw))))

(event `CheckAlert`
  (`BlackboardComponent.SetValueAsBool` (`AIBlueprintHelperLibrary.GetBlackboard` (`AIBlueprintHelperLibrary.GetAIController` self)) "Alerted?" false))

(event `JumpAttack`
  (`|ExecutionSequence`
    (:`then_1`
      (`PrimitiveComponent.SetMaterial` (`self.Mesh`) 0 "/Game/Enemies/FrostSlime/Visuals/AttackFlash.AttackFlash")
      (`KismetSystemLibrary.Delay` 0.8)
      (`PrimitiveComponent.SetMaterial` (`self.Mesh`) 0 "/Game/Enemies/FrostSlime/Visuals/Slime1.Slime1")
      (set `self.IsAttacking` true)
      (`self.LaunchCharacter` (0.0 0.0 300.0))
      (`KismetSystemLibrary.Delay` 0.2)
      (`self.LaunchCharacter` (* (`KismetMathLibrary.GetForwardVector` (`self.K2_GetActorRotation`)) (`self.JumpDistance`)))
      (`KismetSystemLibrary.Delay` 1.5)
      (set `self.IsAttacking` false))))

(event `self.ReceiveDestroyed`
  (`/Game/BlueprintLibary/AIFuncation_BPL.AddToArray` self (`self.SpawnLocation`)))

(event `ShowAlert`
  (`/Engine/EditorBlueprintResources/StandardMacros.DoOnce` false :!label _label_2
    (:`Completed`
      (`SceneComponent.SetHiddenInGame` (`self.Alerted`) false false)
      (`KismetSystemLibrary.Delay` 1.0)
      (`SceneComponent.SetHiddenInGame` (`self.Alerted`) true false))))

(event `Reset Alert`
  (goto _label_2 :!via `Reset`))

(fn `UserConstructionScript`)